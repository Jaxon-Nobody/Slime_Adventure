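; BP_MyDamager is a damage volume that hurts the player's BP_SlimeCharacter while it is inside.
; On overlap begin, it checks the player tag, stores the character and applies instant damage, capped at MaxDamage, through ChangeHealth.
; Tick then drains health at DamageRate, scaled by delta time, until the accumulated damage reaches MaxDamage or the player leaves.
; Each re-entry restarts the accumulation from the instant damage.
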(event `self.ReceiveTick`
  (params (DeltaSeconds :type "Float (single-precision)"))
  (if (`self.Inside Volume`)
    (`self.Continue Damamge`)))

(event `self.Collision Volume.OnComponentBeginOverlap`
  (params (OverlappedComponent :type "PrimitiveComponent Object Reference") (OtherActor :type "Actor Object Reference") (OtherComp :type "PrimitiveComponent Object Reference") (OtherBodyIndex :type Integer) (bFromSweep :type Boolean) (SweepResult :type "HitResult Structure (by ref)"))
  (if (`self.ActorHasTag` OtherActor "Tag_Player")
    (bind _asbp_slime_character (cast `/Game/__MyContent/Blueprints/BP_SlimeCharacter` OtherActor))
    (set `self.Inside Volume` true)
    (set `self.Player` _asbp_slime_character)
    (`self.Start Damage`)))

(event `self.Collision Volume.OnComponentEndOverlap`
  (params (OverlappedComponent :type "PrimitiveComponent Object Reference") (OtherActor :type "Actor Object Reference") (OtherComp :type "PrimitiveComponent Object Reference") (OtherBodyIndex :type Integer))
  (if (`self.ActorHasTag` OtherActor "Tag_Player")
    (cast `/Game/__MyContent/Blueprints/BP_SlimeCharacter` OtherActor)
    (set `self.Inside Volume` false)))

(fn `Continue Damamge`
  (bind _returnvalue (* (`self.Damage Rate`) (`GameplayStatics.GetWorldDeltaSeconds`)))
  (if (< (`self.Accum Damage`) (`self.Max Damage`))
    (set `self.Accum Damage` (+ _returnvalue (`self.Accum Damage`))) ; increase accum damage by rate
    (`/Game/__MyContent/Blueprints/BP_SlimeCharacter.Change Health` (`self.Player`) (* _returnvalue -1.0))))

(fn `Start Damage`
  (bind _output_get (set `self.Accum Damage` (`self.Instant Damge`)))
  (if (> _output_get (`self.Max Damage`))
    (set `self.Accum Damage` (`self.Max Damage`)))
  (`/Game/__MyContent/Blueprints/BP_SlimeCharacter.Change Health` (`self.Player`) (* (`self.Accum Damage`) -1.0)))

(fn `UserConstructionScript`)