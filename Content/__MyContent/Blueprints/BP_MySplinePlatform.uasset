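; BP_MySplinePlatform is a moving platform actor that travels along a spline path.
; The construction script applies a configurable static mesh and material to the platform mesh.
; On BeginPlay a timeline starts, and its SplineDistance track, scaled by the spline length, sets the mesh's world position along the spline each update without sweeping.
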(event `Platform Start`
  (bind _spline (`self.Spline`))
  (bind (_direction _spline_distance) (`Timeline|Motion Timeline` :!via `PlayFromStart`)
    (:`Update`
      (`SceneComponent.K2_SetWorldLocation` (`self.Platform Mesh`) (`SplineComponent.GetLocationAtDistanceAlongSpline` _spline (* (`SplineComponent.GetSplineLength` _spline) _spline_distance) "World") false false))))

(event `self.ReceiveBeginPlay`
  (`self.Platform Start`))

(fn `UserConstructionScript`
  (`StaticMeshComponent.SetStaticMesh` (`self.Platform Mesh`) (`self.Static Mesh`))
  (`PrimitiveComponent.SetMaterial` (`self.Platform Mesh`) 0 (`self.Material`)))